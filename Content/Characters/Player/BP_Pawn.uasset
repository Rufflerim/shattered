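; Player pawn that acts as a movable camera rig, with panning, zoom and stepped rotation.
; Axis inputs shift a move target along the actor's forward and right vectors and adjust a clamped zoom target, while rotation key presses add fixed yaw steps to a rotation target.
; Each Tick interpolates actor location, actor rotation and spring arm length toward those targets for smooth motion.
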(event EventTick
  (params (DeltaSeconds :type Float%20%28single-precision%29))
  (CallFunction|CameraZoom DeltaSeconds)
  (CallFunction|CameraMovement DeltaSeconds)
  (CallFunction|CameraRotation DeltaSeconds))

(event EventBeginPlay
  (Variables|Default|SetMoveTarget (Transformation|GetActorLocation))
  (Variables|Default|SetZoomTarget (Variables|/Script/Engine.SpringArmComponent|GetTargetArmLength (Variables|Default|GetSpringArm)))
  (Variables|Default|SetRotationTarget (Transformation|GetActorRotation)))

(event Input|ActionEvents|InputActionInputAction_RotationRight
  (params (Key :type Key%20Structure :default "None"))
  ;[0 0 0] Rotate Camera
  (:Pressed
    (Variables|Default|SetRotationTarget (Math|Rotator|CombineRotators (Variables|Default|GetRotationTarget) (Math|Rotator|MakeRotator 0.0 0.0 (* (Variables|Default|GetRotationSpeed) -1.0))))))

(event Input|ActionEvents|InputActionInputAction_RotationLeft
  (params (Key :type Key%20Structure :default "None"))
  ;[0 0 0] Rotate Camera
  (:Pressed
    (Variables|Default|SetRotationTarget (Math|Rotator|CombineRotators (Variables|Default|GetRotationTarget) (Math|Rotator|MakeRotator 0.0 0.0 (Variables|Default|GetRotationSpeed))))))

(event Input|AxisEvents|InputAxisInputAxis_Zoom
  (params (AxisValue :type Float%20%28single-precision%29))
  ;[0 0 0] Zoom Camera
  (Variables|Default|SetZoomTarget (Math|Float|Clamp(Float) (+ (* AxisValue (Variables|Default|GetZoomSpeed)) (Variables|Default|GetZoomTarget)) (Variables|Default|GetZoomMin) (Variables|Default|GetZoomMax))))

(event Input|AxisEvents|InputAxisInputAxis_Forward
  (params (AxisValue :type Float%20%28single-precision%29))
  ;[0 0 0] Move Camera
  (Variables|Default|SetMoveTarget (+ (Variables|Default|GetMoveTarget) (* (* AxisValue (Variables|Default|GetMoveSpeed)) (Transformation|GetActorForwardVector)))))

(event Input|AxisEvents|InputAxisInputAxis_Right
  (params (AxisValue :type Float%20%28single-precision%29))
  ;[0 0 0] Move Camera
  (Variables|Default|SetMoveTarget (+ (Variables|Default|GetMoveTarget) (* (* AxisValue (Variables|Default|GetMoveSpeed)) (Transformation|GetActorRightVector)))))

(fn ConstructionScript)

(fn CameraZoom
  (params (DeltaTime :type Float%20%28double-precision%29))
  (bind _springarm (Variables|Default|GetSpringArm))
  (Variables|/Script/Engine.SpringArmComponent|SetTargetArmLength _springarm (Math|Interpolation|FInterpTo (Variables|/Script/Engine.SpringArmComponent|GetTargetArmLength _springarm) (Variables|Default|GetZoomTarget) DeltaTime (Variables|Default|GetZoomInterp))))

(fn CameraMovement
  (params (DeltaTime :type Float%20%28single-precision%29))
  (Transformation|SetActorLocation (Math|Interpolation|VInterpTo (Transformation|GetActorLocation) (Variables|Default|GetMoveTarget) DeltaTime (Variables|Default|GetMoveInterpSpeed)) false false))

(fn CameraRotation
  (params (DeltaTime :type Float%20%28single-precision%29))
  (Transformation|SetActorRotation (Math|Interpolation|RInterpTo (Transformation|GetActorRotation) (Variables|Default|GetRotationTarget) DeltaTime (Variables|Default|GetRotationInterp))))