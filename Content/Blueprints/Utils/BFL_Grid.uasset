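; Blueprint function library of helper utilities for grid math and grid shape lookup.
; It snaps a vector per axis to the matching grid sizes in a second vector, returning separate X, Y and Z values, and tests floats and ints for evenness.
; GetShapeData converts a GridShape enum into a row name to read DT_GridShapeData, printing an on-screen error when the row is missing.
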(fn SnapVectortoVector
  (params (V1 :type Vector) (V2 :type Vector))
  (return (Math|Vector|MakeVector (Math|Float|SnapToGrid(Float) (.x V1) (.x V2)) (Math|Float|SnapToGrid(Float) (.y V1) (.y V2)) (Math|Float|SnapToGrid(Float) (.z V1) (.z V2)))))

(fn IsFloatEven
  (params (Float :type Float%20%28double-precision%29))
  (return (== (Math|Float|%(Float) Float 2.0) 0.0)))

(fn IsIntEven
  (params (Int :type Integer))
  (return (== (Math|Integer|%(Integer) Int 2) 0)))

(fn GetShapeData
  (params (GridShape :type E_GridShape%20Enum :default "NewEnumerator3"))
  (bind _returnvalue (Utilities|String|EnumtoString GridShape))
  (bind _returnvalue_2 (Utilities|GetDataTableRow "/Game/Blueprints/Core/Grid/DT_GridShapeData.DT_GridShapeData" (Utilities|String|StringToName _returnvalue))
    (:then
      (return _returnvalue_2))
    (:RowNotFound
      (Development|PrintString 0 (Utilities|String|Append "Error - Invalid Row Name " _returnvalue) true true "(R=1.000000,G=0.000000,B=0.067223,A=1.000000)" 5.0))))