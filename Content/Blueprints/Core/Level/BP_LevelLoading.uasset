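; BP_LevelLoading manages streaming levels by name, keeping track of one loaded level at a time.
; On BeginPlay it force-loads the level named in LoadedLevel.
; LoadLevel skips repeat requests unless forced, flags the previous streaming level to unload and hide, then stores the new name and flags that level to load and show.
; An invalid new level name prints a red error.
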(event EventBeginPlay
  (CallFunction|LoadLevel (Variables|Default|GetLoadedLevel) true))

(fn ConstructionScript)

(fn LoadLevel
  (params (Level :type String) (Force :type Boolean))
  (bind _returnvalue (Utilities|String|StringToName Level))
  (bind _returnvalue_2 (Class|GameplayStatics|GetStreamingLevel _returnvalue))
  (if (or Force (Utilities|Enum|NotEqual(Enum) Level (Variables|Default|GetLoadedLevel)))
    (Utilities|FlowControl|Sequence
      (:then_0
        (Utilities|IsValid (Class|GameplayStatics|GetStreamingLevel (Utilities|String|StringToName (Variables|Default|GetLoadedLevel)))
          (:Is%20Valid
            (Variables|/Script/Engine.LevelStreaming|SetbShouldBeLoaded (Class|GameplayStatics|GetStreamingLevel (Utilities|String|StringToName (Variables|Default|GetLoadedLevel))) false)
            (Variables|/Script/Engine.LevelStreaming|SetbShouldBeVisible (Class|GameplayStatics|GetStreamingLevel (Utilities|String|StringToName (Variables|Default|GetLoadedLevel))) false))))
      (:then_1
        (Variables|Default|SetLoadedLevel Level)
        (Utilities|IsValid _returnvalue_2
          (:Is%20Valid
            (Variables|/Script/Engine.LevelStreaming|SetbShouldBeLoaded _returnvalue_2 true)
            (Variables|/Script/Engine.LevelStreaming|SetbShouldBeVisible _returnvalue_2 true))
          (:Is%20Not%20Valid
            (Development|PrintString (Utilities|String|Append "Error - LoadLevel - Invalid Level Name: " Level) true true "(R=1.000000,G=0.000000,B=0.004751,A=1.000000)")))))))