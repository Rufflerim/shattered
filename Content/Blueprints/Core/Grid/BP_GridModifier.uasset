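; BP_GridModifier is an editor-visible grid marker with a shape and a type (None, Normal or Obstacle), hidden during play.
; Its construction script pulls the mesh and flat material from the shape data, then sets a filled look with a color chosen by type.
; The mesh overlaps a custom trace channel, and the event graph holds no active logic.
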(event EventBeginPlay)

(event Collision|EventActorBeginOverlap
  (params (OtherActor :type Actor%20Object%20Reference)))

(event EventTick
  (params (DeltaSeconds :type Float%20%28single-precision%29)))

(fn ConstructionScript
  (bind _staticmesh (Variables|Default|GetStaticMesh))
  (bind _shape (Variables|Default|GetShape))
  (bind _data (CallFunction|GetShapeData _shape))
  (Components|StaticMesh|SetStaticMesh _staticmesh (.mesh _data))
  (Rendering|Material|SetMaterial _staticmesh 0 (.flatmaterial _data))
  (Rendering|Material|SetVectorParameterValueonMaterials _staticmesh "Color" (Math|Conversions|ToVector(LinearColor) (Utilities|Select :Index (Variables|Default|GetType) :NewEnumerator0 "" :NewEnumerator1 "(R=1.000000,G=1.000000,B=1.000000,A=1.000000)" :NewEnumerator2 "(R=0.932292,G=0.101969,B=0.101969,A=1.000000)")))
  (Rendering|Material|SetScalarParameterValueonMaterials _staticmesh "IsFilled" 1.0)
  (Collision|SetCollisionResponsetoChannel (Variables|Default|GetStaticMesh) "ECC_GameTraceChannel1" "ECR_Overlap")
  (Rendering|SetActorHiddenInGame true))