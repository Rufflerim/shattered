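; BP_GridMeshInst is a grid actor that draws one mesh type at many grid indices through a single InstancedStaticMesh component.
; InitGridMeshInst sets the mesh, material, Color parameter and collision mode.
; AddInstance replaces any existing instance at that index, using a component-local transform.
; A parallel InstanceIndices array maps grid indices to instance positions for removal and clearing; Tick is disabled at BeginPlay.
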(event EventBeginPlay
  (Actor|Tick|SetActorTickEnabled false))

(event Collision|EventActorBeginOverlap
  (params (OtherActor :type Actor%20Object%20Reference)))

(event EventTick
  (params (DeltaSeconds :type Float%20%28single-precision%29)))

(fn ConstructionScript)

(fn AddInstance
  (params (Index :type Int%20Point%20Structure%20%28by%20ref%29) (Transform :type Transform%20%28by%20ref%29))
  (CallFunction|RemoveInstance Index)
  (Components|InstancedStaticMesh|AddInstance (Variables|Default|GetInstancedStaticMesh) Transform false)
  (Utilities|Array|Add (Variables|Default|GetInstanceIndices) Index))

(fn RemoveInstance
  (params (Index :type Int%20Point%20Structure%20%28by%20ref%29))
  (bind _instanceindices (Variables|Default|GetInstanceIndices))
  (if (Utilities|Array|ContainsItem _instanceindices Index)
    (Class|InstancedStaticMeshComponent|RemoveInstance (Variables|Default|GetInstancedStaticMesh) (Utilities|Array|FindItem _instanceindices Index))
    (Utilities|Array|RemoveItem (Variables|Default|GetInstanceIndices) Index)))

(fn ClearInstances
  (Components|InstancedStaticMesh|ClearInstances (Variables|Default|GetInstancedStaticMesh))
  (Utilities|Array|Clear (Variables|Default|GetInstanceIndices)))

(fn InitGridMeshInst
  (params (NewMesh :type Static%20Mesh%20Object%20Reference) (Material :type Material%20Interface%20Object%20Reference) (Color :type Linear%20Color%20Structure) (CollisionType :type ECollisionEnabled%20Enum :default "NoCollision"))
  (bind _instancedstaticmesh (Variables|Default|GetInstancedStaticMesh))
  (Components|StaticMesh|SetStaticMesh _instancedstaticmesh NewMesh)
  (Rendering|Material|SetMaterial _instancedstaticmesh 0 Material)
  (Rendering|Material|SetVectorParameterValueonMaterials _instancedstaticmesh "Color" (Math|Conversions|ToVector(LinearColor) Color))
  (Collision|SetCollisionEnabled _instancedstaticmesh CollisionType))