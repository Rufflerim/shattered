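; BP_GridPathfinding runs A* searches between tiles on square, hexagon or triangle grids, filtered by tile type and height step.
; FindPath seeds a cost-sorted open list, expands the cheapest tile with shape-specific neighbours and heuristics, and retraces the path once the target is discovered.
; Sorting penalises diagonal steps to break ties.
; Searches run instantly or across delayed iterations with an optional per-frame time budget, reporting progress and results through callbacks.
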(event Custom|FindPathWithDelay
  (Utilities|FlowControl|Sequence
    (:then_0
      (goto _label_3 Open))
    (:then_1
      (Variables|Default|SetLoopStartTime (Math|DateTime|Now) :!label _label)
      (if (> (Utilities|Array|Length (Variables|Default|GetDiscoveredTileIndices)) 0) :!label _label_2
        (bind _foundtargettile (Path|AnalyseNextDiscoveredTile))
        (if _foundtargettile
          (bind _path (Path|RetrievePath))
          (Default|CallOnPathfindingCompleted _path)
          (else
            (if (> (Variables|Default|GetMaxMsPerFrame) 0.0) ; Do we have a tiome limit?
              (if (< (Class|KismetMathLibrary|GetTotalMilliseconds (- (Math|DateTime|Now) (Variables|Default|GetLoopStartTime))) (Variables|Default|GetMaxMsPerFrame)) ; Do we have a tiome limit?
                (goto _label_2)
                (else
                  _)))
            (Utilities|FlowControl|RetriggerableDelay (Variables|Default|GetDelayBetweenIterations))
            (Utilities|FlowControl|Gate true :!label _label_3
              (:Exit
                (goto _label)))))
        (else
          (Default|CallOnPathfindingCompleted (Utilities|Array|MakeArray "")))))))

(event Custom|CloseDelayGate
  (Utilities|FlowControl|Gate true) ; enters at Close
)

(event EventBeginPlay)

(event Collision|EventActorBeginOverlap
  (params (OtherActor :type Actor%20Object%20Reference)))

(event EventTick
  (params (DeltaSeconds :type Float%20%28single-precision%29)))

(fn ConstructionScript)

(fn GetValidTileNeighbours
  (params (Index :type Int%20Point%20Structure) (IncludeDiagonals :type Boolean) (ValidTileTypes :type Array%20of%20E_TileType%20Enums :default "NewEnumerator0"))
  (LocalVariables|SetInputData (.Value (Utilities|Map|Find (Variables|/Game/Blueprints/Core/Grid/BP_Grid.BP_Grid_C|GetGridTiles (Variables|Default|GetGrid)) Index)))
  (bind _neighbours (Neighbours|GetNeighboursIndices Index IncludeDiagonals))
  (for _array_element _neighbours
    (LocalVariables|SetTileData (.Value (Utilities|Map|Find (Variables|/Game/Blueprints/Core/Grid/BP_Grid.BP_Grid_C|GetGridTiles (Variables|Default|GetGrid)) _array_element)))
    (if (Utilities|Array|ContainsItem ValidTileTypes (.type (LocalVariables|GetTileData)))
      (if (<= (Math|Float|Absolute(Float) (- (.z (.location (.transform (LocalVariables|GetTileData)))) (.z (.location (.transform (LocalVariables|GetInputData)))))) (.z (Variables|/Game/Blueprints/Core/Grid/BP_Grid.BP_Grid_C|GetGridTileSize (Variables|Default|GetGrid))))
        (Utilities|Array|Add (LocalVariables|GetValidIndices) (Utilities|Struct|MakeS_PathfindingData (.index (LocalVariables|GetTileData)) Index (Utilities|Select :Index (.type (LocalVariables|GetTileData)) :NewEnumerator0 0 :NewEnumerator1 1 :NewEnumerator2 0 :NewEnumerator3 2 :NewEnumerator4 3 :NewEnumerator5 1) 999999 999999)))))
  (return (LocalVariables|GetValidIndices)))

(fn GetNeighboursIndicesSquare
  (params (Index :type Int%20Point%20Structure) (IncludeDiagonals :type Boolean))
  (bind _intpoint (Utilities|Struct|MakeIntPoint 1 0))
  (bind _intpoint_2 (Utilities|Struct|MakeIntPoint 0 1))
  (bind _intpoint_3 (Utilities|Struct|MakeIntPoint -1 0))
  (bind _intpoint_4 (Utilities|Struct|MakeIntPoint 0 -1))
  (bind _returnvalue (+ Index _intpoint))
  (bind _returnvalue_2 (+ Index _intpoint_2))
  (bind _returnvalue_3 (+ Index _intpoint_3))
  (bind _returnvalue_4 (+ Index _intpoint_4))
  (bind _array (Utilities|Array|MakeArray _returnvalue _returnvalue_2 _returnvalue_3 _returnvalue_4))
  (if IncludeDiagonals
    (bind _output_get (LocalVariables|SetTempNeighbours _array))
    (Utilities|Array|AppendArray _output_get (Utilities|Array|MakeArray (+ Index (Utilities|Struct|MakeIntPoint 1 1)) (+ Index (Utilities|Struct|MakeIntPoint -1 1)) (+ Index (Utilities|Struct|MakeIntPoint 1 -1)) (+ Index (Utilities|Struct|MakeIntPoint -1 -1))))
    (return (LocalVariables|GetTempNeighbours))
    (else
      (return _array))))

(fn GetNeighboursIndicesHexagon
  (params (Index :type Int%20Point%20Structure))
  (return (Utilities|Array|MakeArray (+ Index (Utilities|Struct|MakeIntPoint 1 1)) (+ Index (Utilities|Struct|MakeIntPoint 0 2)) (+ Index (Utilities|Struct|MakeIntPoint -1 1)) (+ Index (Utilities|Struct|MakeIntPoint -1 -1)) (+ Index (Utilities|Struct|MakeIntPoint 0 -2)) (+ Index (Utilities|Struct|MakeIntPoint 1 -1)))))

(fn GetNeighboursIndicesTriangle
  (params (Index :type Int%20Point%20Structure) (IncludeDiagonals :type Boolean))
  (LocalVariables|SetTempNeighbours (Utilities|Array|MakeArray (+ Index (Utilities|Struct|MakeIntPoint 0 -1)) (+ Index (Utilities|Struct|MakeIntPoint 0 1))))
  (if (== (CallFunction|IsIntEven (.x Index)) (CallFunction|IsIntEven (.y Index)))
    (Utilities|Array|Add (LocalVariables|GetTempNeighbours) (+ Index (Utilities|Struct|MakeIntPoint -1 0)))
    (else
      (Utilities|Array|Add (LocalVariables|GetTempNeighbours) (+ Index (Utilities|Struct|MakeIntPoint 1 0)))))
  (if IncludeDiagonals
    (if (== (CallFunction|IsIntEven (.x Index)) (CallFunction|IsIntEven (.y Index)))
      (Utilities|Array|AppendArray (LocalVariables|GetTempNeighbours) (Utilities|Array|MakeArray (+ Index (Utilities|Struct|MakeIntPoint 1 0)) (+ Index (Utilities|Struct|MakeIntPoint -1 2)) (+ Index (Utilities|Struct|MakeIntPoint -1 -2))))
      (else
        (Utilities|Array|AppendArray (LocalVariables|GetTempNeighbours) (Utilities|Array|MakeArray (+ Index (Utilities|Struct|MakeIntPoint -1 0)) (+ Index (Utilities|Struct|MakeIntPoint 1 2)) (+ Index (Utilities|Struct|MakeIntPoint 1 -2))))))
    (return (LocalVariables|GetTempNeighbours))
    (else
      (return (LocalVariables|GetTempNeighbours)))))

(fn GetNeighboursIndices
  (params (Index :type Int%20Point%20Structure) (IncludeDiagonals :type Boolean))
  (switch Utilities|FlowControl|Switch|SwitchonE_GridShape (Variables|/Game/Blueprints/Core/Grid/BP_Grid.BP_Grid_C|GetGridShape (Variables|Default|GetGrid))
    (:NewEnumerator0
      (return (Neighbours|GetNeighboursIndicesHexagon Index)))
    (:NewEnumerator1
      (return (Neighbours|GetNeighboursIndicesSquare Index IncludeDiagonals)))
    (:NewEnumerator2
      (return (Neighbours|GetNeighboursIndicesTriangle Index IncludeDiagonals)))))

(fn FindPath
  (params (Start :type Int%20Point%20Structure) (Target :type Int%20Point%20Structure) (Diagonals :type Boolean) (Valid%20Tile%20Types :type Array%20of%20E_TileType%20Enums :default "NewEnumerator0") (Delay :type Float%20%28double-precision%29) (MaxMsPerFrame :type Float%20%28double-precision%29))
  (bind _array (Utilities|Array|MakeArray ""))
  (bind _array_2 (Utilities|Array|MakeArray ""))
  (Variables|Default|SetStartIndex Start)
  (Variables|Default|SetTargetIndex Target)
  (Variables|Default|SetIncludeDiagonals Diagonals)
  (Variables|Default|SetValid%20Tile%20Types Valid%20Tile%20Types)
  (Variables|Default|SetDelayBetweenIterations Delay)
  (Variables|Default|SetMaxMsPerFrame MaxMsPerFrame)
  (CallFunction|CloseDelayGate)
  (Path|ClearGeneratedData)
  (bind _isvalid (Path|IsInputDataValid))
  (if _isvalid
    (Path|DiscoverTile (Utilities|Struct|MakeS_PathfindingData (Variables|Default|GetStartIndex) "(X=-999,Y=-999)" 1 0 (Path|GetMinimumCostBetweenTwoTiles (Variables|Default|GetStartIndex) (Variables|Default|GetTargetIndex) (Variables|Default|GetIncludeDiagonals))))
    (if (<= (Variables|Default|GetDelayBetweenIterations) 0.0)
      ;[1 1 1] Complete find path
      (while (> (Utilities|Array|Length (Variables|Default|GetDiscoveredTileIndices)) 0)
        (bind _foundtargettile (Path|AnalyseNextDiscoveredTile))
        (if _foundtargettile
          (bind _path (Path|RetrievePath))
          (Default|CallOnPathfindingCompleted _path)
          (return _path)))
      (Default|CallOnPathfindingCompleted _array_2)
      (return _array_2)
      (else
        ;[1 1 1] Progressive find path
        (CallFunction|FindPathwithDelay)
        (return (Utilities|Array|MakeArray ""))))
    (else
      (Default|CallOnPathfindingCompleted _array)
      (return _array))))

(fn IsInputDataValid
  (if (!= (Variables|Default|GetStartIndex) "")
    (if (Default|IsTileWalkable (Variables|Default|GetGrid) (Variables|Default|GetStartIndex))
      (if (Default|IsTileWalkable (Variables|Default|GetGrid) (Variables|Default|GetTargetIndex))
        ;[1 1 1] Dont compute path if target tile type is not a valid type
        (if (Utilities|Array|ContainsItem (Variables|Default|GetValid%20Tile%20Types) (.Type (Utilities|Struct|BreakS_TileData (.Value (Utilities|Map|Find (Variables|/Game/Blueprints/Core/Grid/BP_Grid.BP_Grid_C|GetGridTiles (Variables|Default|GetGrid)) (Variables|Default|GetTargetIndex))))))
          (return true))
        (else
          (return false)))
      (else
        (return false)))
    (else
      (return false))))

(fn DiscoverTile
  (params (TilePathData :type S%20Pathfinding%20Data%20Structure))
  (bind _index (Utilities|Struct|BreakS_PathfindingData TilePathData))
  (Utilities|Map|Add (Variables|Default|GetPathfindingData) _index TilePathData)
  (Path|InsertTileOrderedinDiscoveredArray TilePathData)
  (Default|CallOnPathfindingDataUpdated _index))

(fn GetMinimumCostBetweenTwoTiles
  (params (Index1 :type Int%20Point%20Structure) (Index2 :type Int%20Point%20Structure) (Diagonals :type Boolean))
  (bind _returnvalue (- Index1 Index2))
  (bind _returnvalue_2 (< (.x Index2) (.x Index1)))
  (bind _returnvalue_3 (< (.x Index2) (.x Index1)))
  (bind _returnvalue_4 (- Index1 Index2))
  (bind _returnvalue_5 (- Index1 Index2))
  (bind _returnvalue_6 (- Index1 Index2))
  (bind _returnvalue_7 (Math|Integer|SelectInt -1 1 _returnvalue_2))
  (bind _returnvalue_8 (Math|Integer|Absolute(Integer) (.x _returnvalue)))
  (bind _returnvalue_9 (Math|Integer|Absolute(Integer) (.x _returnvalue_5)))
  (bind _returnvalue_10 (Math|Integer|Absolute(Integer) (.y _returnvalue_5)))
  (switch Utilities|FlowControl|Switch|SwitchonE_GridShape (Variables|/Game/Blueprints/Core/Grid/BP_Grid.BP_Grid_C|GetGridShape (Variables|Default|GetGrid))
    (:NewEnumerator0
      (return (+ _returnvalue_8 (Math|Integer|Max(Integer) (/ (- (Math|Integer|Absolute(Integer) (.y _returnvalue)) _returnvalue_8) 2)))))
    (:NewEnumerator1
      (if Diagonals
        (return (Math|Integer|Max(Integer) _returnvalue_9 _returnvalue_10))
        (else
          (return (+ _returnvalue_9 _returnvalue_10)))))
    (:NewEnumerator2
      (if Diagonals
        (return (+ (Math|Integer|Absolute(Integer) (.x _returnvalue_6)) (Math|Integer|Absolute(Integer) (.y _returnvalue_6))))
        (else
          (LocalVariables|SetX (Math|Integer|Absolute(Integer) (.x _returnvalue_4)))
          (LocalVariables|SetY (Math|Integer|Absolute(Integer) (.y _returnvalue_4)))
          (if (select (== (CallFunction|IsIntEven (.x Index1)) (CallFunction|IsIntEven (.y Index1))) (select _returnvalue_3 (<= (- (LocalVariables|GetX) 1) (LocalVariables|GetY)) (<= (LocalVariables|GetX) (LocalVariables|GetY))) (select _returnvalue_3 (<= (LocalVariables|GetX) (LocalVariables|GetY)) (<= (- (LocalVariables|GetX) 1) (LocalVariables|GetY)))) ; Is part of the normal zone?
            (return (+ (LocalVariables|GetX) (LocalVariables|GetY)))
            (elif (== (CallFunction|IsIntEven (LocalVariables|GetX)) (CallFunction|IsIntEven (LocalVariables|GetY))) ; Is facing up?
              (return (* (LocalVariables|GetX) 2))
              (else
                (return (+ (* (LocalVariables|GetX) 2) (Math|Integer|SelectInt _returnvalue_7 (* _returnvalue_7 -1) (== (CallFunction|IsIntEven (.x Index1)) (CallFunction|IsIntEven (.y Index1))))))))))))))

(fn AnalyseNextDiscoveredTile
  (bind _tilepathdata (Path|PullCheapestTileOutOfDiscoveredList))
  (bind _output_get (Variables|Default|SetCurrentDiscoveredTile _tilepathdata))
  (Default|CallOnPathfindingDataUpdated (.Index (Utilities|Struct|BreakS_PathfindingData _output_get)))
  (bind _neighbours (Neighbours|GetValidTileNeighbours (.Index (Utilities|Struct|BreakS_PathfindingData _output_get)) (Variables|Default|GetIncludeDiagonals) (Variables|Default|GetValid%20Tile%20Types)))
  (bind _output_get_2 (Variables|Default|SetCurrentNeighbours _neighbours))
  (while (> (Utilities|Array|Length _output_get_2) 0)
    (bind _istargettile (Path|DiscoverNextNeighbour))
    (if _istargettile
      (return true)))
  (return false))

(fn RetrievePath
  (bind _output_get (LocalVariables|SetCurrent (Variables|Default|GetTargetIndex)))
  (while (!= _output_get (Variables|Default|GetStartIndex))
    (Utilities|Array|Add (LocalVariables|GetInvertedPath) (LocalVariables|GetCurrent))
    (LocalVariables|SetCurrent (.PreviousIndex (Utilities|Struct|BreakS_PathfindingData (.Value (Utilities|Map|Find (Variables|Default|GetPathfindingData) (LocalVariables|GetCurrent)))))))
  (Utilities|Array|Reverse (LocalVariables|GetInvertedPath))
  (return (LocalVariables|GetInvertedPath)))

(fn PullCheapestTileOutOfDiscoveredList
  (LocalVariables|SetTileIndex (Utilities|Array|Get(acopy) (Variables|Default|GetDiscoveredTileIndices)))
  (Utilities|Array|RemoveIndex (Variables|Default|GetDiscoveredTileSortingCosts))
  (Utilities|Array|RemoveIndex (Variables|Default|GetDiscoveredTileIndices))
  (Utilities|Array|Add (Variables|Default|GetAnalysedTileIndices) (LocalVariables|GetTileIndex))
  (return (.Value (Utilities|Map|Find (Variables|Default|GetPathfindingData) (LocalVariables|GetTileIndex)))))

(fn DiscoverNextNeighbour
  (Variables|Default|SetCurrentNeighbour (Utilities|Array|Get(acopy) (Variables|Default|GetCurrentNeighbours)))
  (Utilities|Array|RemoveIndex (Variables|Default|GetCurrentNeighbours))
  (if (not (Utilities|Array|ContainsItem (Variables|Default|GetAnalysedTileIndices) (.Index (Utilities|Struct|BreakS_PathfindingData (Variables|Default|GetCurrentNeighbour)))))
    (LocalVariables|SetCostFromStart (+ (.CostFromStart (Utilities|Struct|BreakS_PathfindingData (Variables|Default|GetCurrentDiscoveredTile))) (.CostToEnterTile (Utilities|Struct|BreakS_PathfindingData (Variables|Default|GetCurrentNeighbour)))))
    (bind _output_get (LocalVariables|SetIndexInDiscovered (Utilities|Array|FindItem (Variables|Default|GetDiscoveredTileIndices) (.Index (Utilities|Struct|BreakS_PathfindingData (Variables|Default|GetCurrentNeighbour))))))
    (if (== _output_get -1)
      _
      (else
        (bind _output_get_2 (Variables|Default|SetCurrentNeighbour (.Value (Utilities|Map|Find (Variables|Default|GetPathfindingData) (.Index (Utilities|Struct|BreakS_PathfindingData (Variables|Default|GetCurrentNeighbour)))))))
        (if (< (LocalVariables|GetCostFromStart) (.CostFromStart (Utilities|Struct|BreakS_PathfindingData _output_get_2)))
          (Utilities|Array|RemoveIndex (Variables|Default|GetDiscoveredTileIndices) (LocalVariables|GetIndexInDiscovered))
          (Utilities|Array|RemoveIndex (Variables|Default|GetDiscoveredTileSortingCosts) (LocalVariables|GetIndexInDiscovered))
          (else
            (return false)))))
    (Path|DiscoverTile (Utilities|Struct|MakeS_PathfindingData (.Index (Utilities|Struct|BreakS_PathfindingData (Variables|Default|GetCurrentNeighbour))) (.Index (Utilities|Struct|BreakS_PathfindingData (Variables|Default|GetCurrentDiscoveredTile))) (.CostToEnterTile (Utilities|Struct|BreakS_PathfindingData (Variables|Default|GetCurrentNeighbour))) (LocalVariables|GetCostFromStart) (Path|GetMinimumCostBetweenTwoTiles (.Index (Utilities|Struct|BreakS_PathfindingData (Variables|Default|GetCurrentNeighbour))) (Variables|Default|GetTargetIndex) (Variables|Default|GetIncludeDiagonals))))
    (if (Class|KismetMathLibrary|EqualIntPointIntPoint (.Index (Utilities|Struct|BreakS_PathfindingData (Variables|Default|GetCurrentNeighbour))) (Variables|Default|GetTargetIndex))
      (return true)
      (else
        (return false)))
    (else
      (return false))))

(fn InsertTileOrderedinDiscoveredArray
  (params (TileData :type S%20Pathfinding%20Data%20Structure))
  (bind _discoveredtilesortingcosts (Variables|Default|GetDiscoveredTileSortingCosts))
  (LocalVariables|SetSortingCost (Path|GetTileSortingCost TileData))
  (if (== (Utilities|Array|Length (Variables|Default|GetDiscoveredTileSortingCosts)) 0)
    ;[1 1 1] When array is empty, just add data
    (Utilities|Array|Add (Variables|Default|GetDiscoveredTileSortingCosts) (LocalVariables|GetSortingCost) :!label _label)
    (Utilities|Array|Add (Variables|Default|GetDiscoveredTileIndices) (.Index (Utilities|Struct|BreakS_PathfindingData TileData)))
    (else
      ;[1 1 1] Optimization: if sorting cost is already bigger, just add at the end
      (if (>= (LocalVariables|GetSortingCost) (Utilities|Array|Get(acopy) _discoveredtilesortingcosts (Utilities|Array|LastIndex _discoveredtilesortingcosts)))
        (goto _label)
        (else
          ;[1 1 1] Insert at right position
          (bind (_array_element _array_index) (Utilities|Array|ForEachLoopwithBreak (Variables|Default|GetDiscoveredTileSortingCosts) :!label _label_2)
            (:LoopBody
              (if (>= _array_element (LocalVariables|GetSortingCost))
                (Utilities|Array|Insert (Variables|Default|GetDiscoveredTileSortingCosts) (LocalVariables|GetSortingCost) _array_index)
                (Utilities|Array|Insert (Variables|Default|GetDiscoveredTileIndices) (.Index (Utilities|Struct|BreakS_PathfindingData TileData)) _array_index)
                (goto _label_2 Break)))))))))

(fn ClearGeneratedData
  (Utilities|Map|Clear (Variables|Default|GetPathfindingData))
  (Utilities|Array|Clear (Variables|Default|GetDiscoveredTileSortingCosts))
  (Utilities|Array|Clear (Variables|Default|GetDiscoveredTileIndices))
  (Utilities|Array|Clear (Variables|Default|GetAnalysedTileIndices))
  (Default|CallOnPathfindingDataCleared))

(fn IsDiagonal
  (params (Index1 :type Int%20Point%20Structure) (Index2 :type Int%20Point%20Structure))
  (bind _neighbours (Neighbours|GetNeighboursIndices Index1 false))
  (return (not (Utilities|Array|ContainsItem _neighbours Index2))))

(fn GetTileSortingCost
  (params (TileData :type S%20Pathfinding%20Data%20Structure%20%28by%20ref%29))
  (bind (_index _previousindex) (Utilities|Struct|BreakS_PathfindingData TileData))
  (bind (_index_2 _previousindex_2 _costtoentertile _costfromstart _minimumcosttotarget) (Utilities|Struct|BreakS_PathfindingData TileData))
  (return (+ (* (+ _costfromstart _minimumcosttotarget) 2) (Path|IsDiagonal _index _previousindex))))