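; Grid actor that builds a square, hexagon or triangle tile grid around its location in the construction script, using one instanced static mesh.
; SpawnGrid clears old instances, takes mesh and material from DT_GridShapeData by shape, then snaps the center and derives the bottom-left corner.
; Tiles are placed from that corner with per-shape spacing.
; Hexagons use doubled Y indices with alternating offsets, while triangles flip yaw by index parity.
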(event EventBeginPlay)

(event Collision|EventActorBeginOverlap
  (params (OtherActor :type Actor%20Object%20Reference)))

(event EventTick
  (params (DeltaSeconds :type Float%20%28single-precision%29)))

(fn ConstructionScript
  (CallFunction|SpawnGrid (Transformation|GetActorLocation) (Variables|Default|GetGridTileSize) (Variables|Default|GetGridTileCount) (Variables|Default|GetGridShape)))

(fn SpawnGrid
  (params (CenterLocation :type Vector) (TileSize :type Vector) (TileCount :type Vector%202D%20Structure) (Shape :type E_GridShape%20Enum :default "NewEnumerator3"))
  (bind (_x _y) (Math|Vector2D|BreakVector2D TileCount))
  (bind _returnvalue (CallFunction|GetCurrentShapeData))
  (bind _instancedstaticmesh (Variables|Default|GetInstancedStaticMesh))
  (bind (_meshsize _mesh _materialinstance _flatmesh _flatbordermaterial) (Utilities|Struct|BreakS_GridShapeData _returnvalue))
  ;[0 0 0] Setup grid config
  (Variables|Default|SetGridCenterLocation CenterLocation)
  (Variables|Default|SetGridTileSize TileSize)
  (Variables|Default|SetGridShape Shape)
  (Variables|Default|SetGridTileCount (Math|Vector2D|MakeVector2D (Math|Conversions|ToFloat(Integer) (Math|Float|Round _x)) (Math|Conversions|ToFloat(Integer) (Math|Float|Round _y))))
  (CallFunction|DestroyGrid)
  (Utilities|FlowControl|Sequence
    (:then_0
      ;[0 0 0] Set meshes and material from data table
      (Components|StaticMesh|SetStaticMesh _instancedstaticmesh _flatmesh)
      (Rendering|Material|SetMaterial _instancedstaticmesh 0 _flatbordermaterial))
    (:then_1
      ;[0 0 0] Set grid position and compute bottom left
      (bind (_center _bottomleft) (CallFunction|CalculateCenterandBottomLeft))
      (Variables|Default|SetGridBottomLeftCornerLocation _bottomleft)
      (Variables|Default|SetGridCenterLocation _center))
    (:then_2
      ;[0 0 0] Create grid tiles from bottom left
      (for _index (range 0 (- (Math|Float|Round (.x (Variables|Default|GetGridTileCount))) 1))
        (LocalVariables|SetX _index)
        (if (Utilities|Enum|NotEqual(Enum) (Variables|Default|GetGridShape) "NewEnumerator0")
          (for _index_2 (range 0 (- (Math|Float|Round (.y (Variables|Default|GetGridTileCount))) 1))
            (LocalVariables|SetY _index_2)
            (LocalVariables|SetIndex (Math|Vector2D|MakeVector2D (Math|Conversions|ToFloat(Integer) (LocalVariables|GetX)) (Math|Conversions|ToFloat(Integer) (LocalVariables|GetY))))
            (LocalVariables|SetTileTransform (Math|Transform|MakeTransform (CallFunction|GetTileLocationfromGridIndex (LocalVariables|GetIndex)) (CallFunction|GetTileRotationfromGridIndex (LocalVariables|GetIndex)) (/ (Variables|Default|GetGridTileSize) (.MeshSize (Utilities|Struct|BreakS_GridShapeData (CallFunction|GetCurrentShapeData))))))
            (Components|InstancedStaticMesh|AddInstance (Variables|Default|GetInstancedStaticMesh) (LocalVariables|GetTileTransform) true))
          (else
            (for _index_3 (range (Math|Integer|SelectInt 0 1 (CallFunction|IsIntEven (LocalVariables|GetX))) (- (* (Math|Float|Round (.y (Variables|Default|GetGridTileCount))) 2) 1))
              (LocalVariables|SetY _index_3)
              (Utilities|FlowControl|Sequence
                (:then_0
                  (LocalVariables|SetIndex (Math|Vector2D|MakeVector2D (Math|Conversions|ToFloat(Integer) (LocalVariables|GetX)) (Math|Conversions|ToFloat(Integer) (LocalVariables|GetY))))
                  (LocalVariables|SetTileTransform (Math|Transform|MakeTransform (CallFunction|GetTileLocationfromGridIndex (LocalVariables|GetIndex)) (CallFunction|GetTileRotationfromGridIndex (LocalVariables|GetIndex)) (/ (Variables|Default|GetGridTileSize) (.MeshSize (Utilities|Struct|BreakS_GridShapeData (CallFunction|GetCurrentShapeData))))))
                  (Components|InstancedStaticMesh|AddInstance (Variables|Default|GetInstancedStaticMesh) (LocalVariables|GetTileTransform) true))
                (:then_1
                  (Math|Integer|IncrementInt _index_3))))))))))

(fn GetCurrentShapeData
  (bind _gridshape (Variables|Default|GetGridShape))
  (bind _returnvalue (Utilities|String|EnumtoString _gridshape))
  (bind _returnvalue_2 (Utilities|GetDataTableRow "/Game/Blueprints/Grid/DT_GridShapeData.DT_GridShapeData" (Utilities|String|StringToName _returnvalue))
    (:then
      (return _returnvalue_2))
    (:RowNotFound
      (Development|PrintString (Utilities|String|Append "Error - Invalid Row Name " _returnvalue) true true "(R=1.000000,G=0.000000,B=0.067223,A=1.000000)" 5.0))))

(fn DestroyGrid
  (Components|InstancedStaticMesh|ClearInstances (Variables|Default|GetInstancedStaticMesh)))

(fn CalculateCenterandBottomLeft
  (bind _gridtilesize (Variables|Default|GetGridTileSize))
  (bind _gridtilecount (Variables|Default|GetGridTileCount))
  (bind _gridtilesize_2 (Variables|Default|GetGridTileSize))
  (bind _gridtilecount_2 (Variables|Default|GetGridTileCount))
  (bind _gridtilesize_3 (Variables|Default|GetGridTileSize))
  (bind _gridtilecount_3 (Variables|Default|GetGridTileCount))
  (bind _gridtilecount_4 (Variables|Default|GetGridTileCount))
  (bind _returnvalue (Math|Conversions|ToVector2D(Vector) _gridtilesize_3))
  (bind _returnvalue_2 (Math|Conversions|ToVector2D(Vector) _gridtilesize_2))
  (bind _iseven (CallFunction|IsFloatEven (.y _gridtilecount_4)))
  (bind _iseven_2 (CallFunction|IsFloatEven (.x _gridtilecount_4)))
  (bind _returnvalue_3 (Math|Conversions|ToVector2D(Vector) _gridtilesize))
  (bind _returnvalue_4 (- _gridtilecount_2 (Math|Vector2D|MakeVector2D 1.0 1.0)))
  (bind _returnvalue_5 (/ _gridtilecount_3 "(X=3.000000,Y=2.000000)"))
  (bind _returnvalue_6 (Math|Float|SelectFloat 0.0 1.0 _iseven))
  (bind _returnvalue_7 (Math|Float|SelectFloat 0.0 1.0 _iseven_2))
  (bind _returnvalue_8 (* _returnvalue_5 _returnvalue))
  (bind _returnvalue_9 (/ _returnvalue_4 "(X=2.000000,Y=4.000000)"))
  (bind _returnvalue_10 (* _returnvalue_9 _returnvalue_2))
  (bind _returnvalue_11 (- _gridtilecount (Math|Vector2D|MakeVector2D _returnvalue_7 _returnvalue_6)))
  (bind _returnvalue_12 (/ _returnvalue_11 2.0))
  (bind _returnvalue_13 (* _returnvalue_12 _returnvalue_3))
  (switch Utilities|FlowControl|Switch|SwitchonE_GridShape (Variables|Default|GetGridShape)
    (:NewEnumerator0
      ;[0 0 0] Hexagon center and bottom left
      (LocalVariables|SetC (CallFunction|SnapVectortoVector (Variables|Default|GetGridCenterLocation) (* (Variables|Default|GetGridTileSize) "1.500000,1.000000,1.000000")))
      (return (LocalVariables|GetC) (CallFunction|SnapVectortoVector (- (LocalVariables|GetC) (Math|Vector|MakeVector (.x _returnvalue_8) (.y _returnvalue_8) 0.0)) (* (Variables|Default|GetGridTileSize) "1.500000,1.000000,1.000000"))))
    (:NewEnumerator1
      ;[0 0 0] Square center and bottom left
      ;;[1 1 1] Snap center along tiles
      (LocalVariables|SetC (CallFunction|SnapVectortoVector (Variables|Default|GetGridCenterLocation) (Variables|Default|GetGridTileSize)))
      (return (LocalVariables|GetC) (- (LocalVariables|GetC) (Math|Vector|MakeVector (.x _returnvalue_13) (.y _returnvalue_13) 0.0))))
    (:NewEnumerator2
      ;[0 0 0] Triangle center and bottom left
      (LocalVariables|SetC (CallFunction|SnapVectortoVector (Variables|Default|GetGridCenterLocation) (* (Variables|Default|GetGridTileSize) "2.000000,1.000000,1.000000")))
      (return (LocalVariables|GetC) (CallFunction|SnapVectortoVector (- (LocalVariables|GetC) (Math|Vector|MakeVector (.x _returnvalue_10) (.y _returnvalue_10) 0.0)) (* (Variables|Default|GetGridTileSize) "2.000000,1.000000,1.000000"))))))

(fn GetTileRotationfromGridIndex
  (params (GridIndex :type Vector%202D%20Structure))
  (bind (_x _y) (Math|Vector2D|BreakVector2D GridIndex))
  (if (Utilities|Enum|Equal(Enum) (Variables|Default|GetGridShape) "NewEnumerator2")
    (return (Math|Rotator|MakeRotator 0.0 0.0 (+ (Math|Float|SelectFloat 1.8e+02 0.0 (CallFunction|IsFloatEven _x)) (Math|Float|SelectFloat 1.8e+02 0.0 (CallFunction|IsFloatEven _y)))))
    (else
      (return "0, 0, 0"))))

(fn GetTileLocationfromGridIndex
  (params (GridIndex :type Vector%202D%20Structure))
  (return (+ (Variables|Default|GetGridBottomLeftCornerLocation) (* (Variables|Default|GetGridTileSize) (* GridIndex (Utilities|Select :Index (Variables|Default|GetGridShape) :NewEnumerator3 "(X=1.000000,Y=1.000000)" :NewEnumerator0 "(X=0.750000,Y=0.500000)" :NewEnumerator1 "(X=1.000000,Y=1.000000)" :NewEnumerator2 "(X=1.000000,Y=0.500000)"))))))